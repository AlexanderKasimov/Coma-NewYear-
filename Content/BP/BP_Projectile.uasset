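; BP_Projectile is a colored, glowing projectile that travels in a straight line and damages what it hits.
; BeginPlay applies Color to a dynamic emissive material and the point light.
; Tick moves it by MoveDirection and Speed using a swept SetActorLocation.
; On any actor overlap, it spawns explosion and impact sound effects, sends Damage to actors implementing IDamageable, then destroys itself.
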(event `self.ReceiveBeginPlay`
  (bind _returnvalue (`PrimitiveComponent.CreateDynamicMaterialInstance` (`self.StaticMesh`) 0 "/Game/Materials/Mat_Emissive_Inst1.Mat_Emissive_Inst1" "None"))
  (`MaterialInstanceDynamic.SetVectorParameterValue` _returnvalue "Color" (`self.Color`))
  (`LightComponent.SetLightColor` (`self.PointLight`) (`self.Color`) true))

(event `self.ReceiveTick`
  (params (DeltaSeconds :type "Float (single-precision)"))
  (`self.K2_SetActorLocation` (+ (`self.K2_GetActorLocation`) (* (`self.MoveDirection`) (* (`GameplayStatics.GetWorldDeltaSeconds`) (`self.Speed`)))) true))

(event `self.ReceiveActorBeginOverlap`
  (params (OtherActor :type "Actor Object Reference"))
  (set `self.OverlappedActor` OtherActor)
  (`|ExecutionSequence`
    (:`then_0`
      (`self.HitVFX`))
    (:`then_1`
      (if (`KismetSystemLibrary.DoesImplementInterface` (`self.OverlappedActor`) "/Game/BP/Interface/IDamageable.IDamageable_C")
        (message `/Game/BP/Interface/IDamageable.HandleDamage` (`self.OverlappedActor`) (`self.Damage`))))
    (:`then_2`
      (`self.K2_DestroyActor`))))

(fn `HitVFX`
  (`GameplayStatics.SpawnEmitterAtLocation` "/Game/StarterContent/Particles/P_Explosion.P_Explosion" (`self.K2_GetActorLocation`) (struct) (`KismetMathLibrary.Conv_DoubleToVector` 0.3))
  (`GameplayStatics.SpawnSoundAtLocation` "/Game/Sound/InGameSound/lasgun-impact_Cue.lasgun-impact_Cue" (`self.K2_GetActorLocation`) (struct) 1.0 1.0 0.0 null null))

(fn `UserConstructionScript`)