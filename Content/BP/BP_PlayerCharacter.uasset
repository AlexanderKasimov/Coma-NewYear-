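; Player character Blueprint with movement, look, jump, automatic blaster fire, health and one-time death reported to GM_Test.
; Fire uses timers to enforce fire rate across repeated presses and to repeat while held.
; Each shot traces from the view point, then spawns a BP_Projectile from the muzzle toward the hit.
; A looping timer traces from the camera to drive depth-of-field focal distance, printing it on screen.
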(event `self.ReceiveBeginPlay`
  (set `self.HP` (`self.MaxHP`))
  (`KismetSystemLibrary.K2_SetTimer` null "UpdateDOF" 0.2 true))

(event `InputAxis|MoveForward`
  (params (AxisValue :type "Float (single-precision)"))
  (`PawnMovementComponent.AddInputVector` (`self.CharacterMovement`) (* (`self.GetActorForwardVector`) AxisValue) false))

(event `InputAxis|MoveRight`
  (params (AxisValue :type "Float (single-precision)"))
  (`PawnMovementComponent.AddInputVector` (`self.CharacterMovement`) (* (`self.GetActorRightVector`) AxisValue) false))

(event `InputAxis|LookUp`
  (params (AxisValue :type "Float (single-precision)"))
  (`self.AddControllerPitchInput` AxisValue))

(event `InputAxis|LookRight`
  (params (AxisValue :type "Float (single-precision)"))
  (`self.AddControllerYawInput` AxisValue))

(event `InputAction|Jump`
  (params (Key :type "Key Structure"))
  (:`Pressed`
    (`self.Jump`)))

(event `InputAction|Fire`
  (params (Key :type "Key Structure"))
  (:`Pressed`
    (if (not (`self.isFiring`))
      (`self.BeginStartFire`)))
  (:`Released`
    (`self.StopFire`)))

(event `/Game/BP/Interface/IDamageable.HandleDamage`
  (params (Damage :type "Float (single-precision)"))
  (set `self.HP` (- (`self.HP`) Damage))
  (if (<= (`self.HP`) 0.0)
    (`/Engine/EditorBlueprintResources/StandardMacros.DoOnce` false
      (:`Completed`
        (`self.HandleDeath`)))))

(fn `BeginStartFire`
  (set `self.isFiring` true)
  (bind _returnvalue (`KismetSystemLibrary.K2_SetTimer` null "StartFire" (`KismetMathLibrary.FMax` (- (+ (`self.LastFireTime`) (/ 1.0 (`self.FireRate`))) (`GameplayStatics.GetTimeSeconds`)) 1e-05)))
  (set `self.TH_StartFire` _returnvalue))

(fn `Fire`
  (locals (HitLocation :type "Vector Structure" :default (0.0 0.0 0.0)) (isHitted :type Boolean :default false))
  (bind (_outlocation _outrotation) (`self.GetActorEyesViewPoint`))
  (`|ExecutionSequence`
    (:`then_0`
      (bind (_outhit _returnvalue) (`KismetSystemLibrary.LineTraceSingle` _outlocation (+ _outlocation (* (`KismetMathLibrary.Conv_RotatorToVector` _outrotation) 10000.0)) "TraceTypeQuery1"))
      (bind _output_get (set `local.isHitted` _returnvalue))
      (if _output_get
        (set `local.HitLocation` (`.Location` (`GameplayStatics.BreakHitResult` _outhit)))))
    (:`then_1`
      (`|SpawnActorFromClass` "/Game/BP/BP_Projectile.BP_Projectile_C" (`KismetMathLibrary.MakeTransform` (`SceneComponent.K2_GetComponentLocation` (`self.Muzzle`)) (`SceneComponent.K2_GetComponentRotation` (`self.MuzzleRotation`))) "AlwaysSpawn" "OverrideRootScale" null (select `bool` (`local.isHitted`) :`false` (`KismetMathLibrary.Conv_RotatorToVector` (`.OutRotation` (`self.GetActorEyesViewPoint`))) :`true` (`KismetMathLibrary.Normal` (- (`local.HitLocation`) (`SceneComponent.K2_GetComponentLocation` (`self.Muzzle`))))) (`self.LaserColor`) 50.0 null)
      (set `self.LastFireTime` (`GameplayStatics.GetTimeSeconds`))
      (`GameplayStatics.SpawnSoundAtLocation` "/Game/Sound/InGameSound/blaster_Cue.blaster_Cue" (`SceneComponent.K2_GetComponentLocation` (`self.Muzzle`)) (struct) 1.0 1.0 0.0 null null))))

(fn `HandleDeath`
  (`self.StopFire`)
  (`self.DisableInput` null)
  (`/Game/BP/GM_Test.PlayerDied(F)` (cast `/Game/BP/GM_Test` (`GameplayStatics.GetGameMode`) :!pure true)))

(fn `StartFire`
  (`self.Fire`)
  (bind _returnvalue (`KismetSystemLibrary.K2_SetTimer` null "Fire" (/ 1.0 (`self.FireRate`)) true))
  (set `self.TH_Fire` _returnvalue))

(fn `StopFire`
  (`KismetSystemLibrary.K2_ClearAndInvalidateTimerHandle` (`self.TH_StartFire`))
  (`KismetSystemLibrary.K2_ClearAndInvalidateTimerHandle` (`self.TH_Fire`))
  (set `self.isFiring` false))

(fn `UpdateDOF`
  (bind _camera (`self.Camera`))
  (bind _returnvalue (`SceneComponent.K2_GetComponentLocation` _camera))
  (`|ExecutionSequence`
    (:`then_0`
      (bind (_outhit _returnvalue_2) (`KismetSystemLibrary.LineTraceSingle` _returnvalue (+ _returnvalue (* (`SceneComponent.GetForwardVector` _camera) 10000.0)) "TraceTypeQuery1"))
      (if _returnvalue_2
        (bind _returnvalue_3 (`KismetMathLibrary.VSize` (- (`.Location` (`GameplayStatics.BreakHitResult` _outhit)) (`SceneComponent.K2_GetComponentLocation` (`self.Camera`)))))
        (set `self.FocalDistance` _returnvalue_3)
        (`KismetSystemLibrary.PrintString` (`KismetStringLibrary.Conv_DoubleToString` _returnvalue_3) true false (struct :`G` 0.66 :`B` 1.0 :`A` 1.0) 0.2)
        (else
          (set `self.FocalDistance` 100000.0))))
    (:`then_1`
      (set `CameraComponent.PostProcessSettings` (make `PostProcessSettings` :`DepthOfFieldMethod` "DOFM_CircleDOF" :`DepthOfFieldFstop` 1.25 :`DepthOfFieldFocalDistance` (`self.FocalDistance`)) (`self.Camera`)))))

(fn `UserConstructionScript`)