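; Spherical enemy turret that detects the player by distance, turns to face them and fires laser projectiles.
; Tick runs the range check, recolors the eye's dynamic material and starts or stops a looping fire timer.
; Fire line-traces from the muzzle to aim each spawned BP_Projectile.
; Damage drains HP until death triggers physics, an explosion and delayed removal; GM_Test's player-death event halts firing.
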(event `self.ReceiveBeginPlay`
  (set `self.HP` (`self.MaxHP`))
  (bind _returnvalue (`PrimitiveComponent.CreateDynamicMaterialInstance` (`self.StaticMesh`) 0 "/Game/Materials/Mat_Emissive_Sine.Mat_Emissive_Sine" "None"))
  (set `self.Mat_Eye` _returnvalue)
  (`MaterialInstanceDynamic.SetVectorParameterValue` (`self.Mat_Eye`) "Color" (`self.EyeColor`))
  (add `/Game/BP/GM_Test.PlayerDied` (cast `/Game/BP/GM_Test` (`GameplayStatics.GetGameMode`) :!pure true) (delegate `OnPlayerDeath`)))

(event `OnPlayerDeath`
  (set `self.isPlayerDead` true)
  (`MaterialInstanceDynamic.SetVectorParameterValue` (`self.Mat_Eye`) "Color" (`self.EyeColor`))
  (`self.StopFire`))

(event `self.ReceiveTick`
  (params (DeltaSeconds :type "Float (single-precision)"))
  (if (and (not (`self.isDead`)) (not (`self.isPlayerDead`)))
    (`|ExecutionSequence`
      (:`then_0`
        (`self.DetectPlayer`))
      (:`then_1`
        (if (`self.isPlayerDetected`)
          (`|ExecutionSequence`
            (:`then_0`
              (`self.K2_SetActorRotation` (`KismetMathLibrary.FindLookAtRotation` (`self.K2_GetActorLocation`) (`self.K2_GetActorLocation` (`GameplayStatics.GetPlayerCharacter` 0)))))
            (:`then_1`
              (if (not (`self.isFiring`))
                (`self.StartFire`))))
          (else
            (`self.StopFire`)))))))

(event `/Game/BP/Interface/IDamageable.HandleDamage`
  (params (Damage :type "Float (single-precision)"))
  (set `self.HP` (- (`self.HP`) Damage))
  (if (<= (`self.HP`) 0.0)
    (`/Engine/EditorBlueprintResources/StandardMacros.DoOnce` false
      (:`Completed`
        (`self.HandleDeath`)))))

(fn `DetectPlayer`
  (if (<= (`KismetMathLibrary.VSize` (- (`self.K2_GetActorLocation`) (`self.K2_GetActorLocation` (`GameplayStatics.GetPlayerCharacter` 0)))) (`self.DetectDistance`))
    (set `self.isPlayerDetected` true)
    (`MaterialInstanceDynamic.SetVectorParameterValue` (`self.Mat_Eye`) "Color" (struct :`R` 1.0 :`G` 0.010417 :`B` 0.010417))
    (else
      (set `self.isPlayerDetected` false)
      (`MaterialInstanceDynamic.SetVectorParameterValue` (`self.Mat_Eye`) "Color" (`self.EyeColor`)))))

(fn `Fire`
  (locals (isHitted :type Boolean) (HitLocation :type "Vector Structure"))
  (bind _returnvalue (`SceneComponent.K2_GetComponentLocation` (`self.Muzzle`)))
  ;[1 1 1] Lmao - turret don't have crosshair LOL
  (`|ExecutionSequence`
    (:`then_0`
      (bind (_outhit _returnvalue_2) (`KismetSystemLibrary.LineTraceSingle` _returnvalue (+ _returnvalue (* (`KismetMathLibrary.Conv_RotatorToVector` (`SceneComponent.K2_GetComponentRotation` (`self.MuzzleRotation`))) 10000.0)) "TraceTypeQuery1"))
      (bind _output_get (set `local.isHitted` _returnvalue_2))
      (if _output_get
        (set `local.HitLocation` (`.Location` (`GameplayStatics.BreakHitResult` _outhit)))))
    (:`then_1`
      (`|SpawnActorFromClass` "/Game/BP/BP_Projectile.BP_Projectile_C" (`KismetMathLibrary.MakeTransform` (`SceneComponent.K2_GetComponentLocation` (`self.Muzzle`)) (`SceneComponent.K2_GetComponentRotation` (`self.MuzzleRotation`))) "AlwaysSpawn" "OverrideRootScale" null (select `bool` (`local.isHitted`) :`false` (`KismetMathLibrary.Conv_RotatorToVector` (`SceneComponent.K2_GetComponentRotation` (`self.MuzzleRotation`))) :`true` (`KismetMathLibrary.Normal` (- (`local.HitLocation`) (`SceneComponent.K2_GetComponentLocation` (`self.Muzzle`))))) (`self.LaserColor`) 20.0 null)
      (`GameplayStatics.SpawnSoundAtLocation` "/Game/Sound/InGameSound/blaster_Cue.blaster_Cue" (`SceneComponent.K2_GetComponentLocation` (`self.Muzzle`)) (struct) 1.0 1.0 0.0 null null))))

(fn `HandleDeath`
  (set `self.isDead` true)
  (`self.StopFire`)
  (`MaterialInstanceDynamic.SetVectorParameterValue` :`self` (`self.Mat_Eye`) :`ParameterName` "Color")
  (`PrimitiveComponent.SetSimulatePhysics` (`self.StaticMesh`) true)
  (`GameplayStatics.SpawnEmitterAtLocation` "/Game/StarterContent/Particles/P_Explosion.P_Explosion" (`self.K2_GetActorLocation`) (struct) (`KismetMathLibrary.Conv_DoubleToVector` 3.0))
  (`GameplayStatics.SpawnSoundAtLocation` "/Game/Sound/InGameSound/lasgun-impact_Cue.lasgun-impact_Cue" (`self.K2_GetActorLocation`) (struct) 1.0 0.925378 0.0 null null)
  (`self.SetLifeSpan` 25.0))

(fn `StartFire`
  (set `self.isFiring` true)
  (bind _returnvalue (`KismetSystemLibrary.K2_SetTimer` null "Fire" (/ 1.0 (`self.FireRate`)) true))
  (set `self.TH_Fire` _returnvalue))

(fn `StopFire`
  (`KismetSystemLibrary.K2_ClearAndInvalidateTimerHandle` (`self.TH_Fire`))
  (set `self.isFiring` false))

(fn `UserConstructionScript`)