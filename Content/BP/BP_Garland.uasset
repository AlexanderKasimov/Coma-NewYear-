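; BP_Garland is a decorative light garland actor, built procedurally in its construction script.
; It spawns Count small static mesh components at even intervals along local X across the float Curve's time range, using the curve value as each one's height.
; Each mesh gets a dynamic instance of an emissive sine material, with its Color parameter cycling through red, blue, green and yellow by index.
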(fn `UserConstructionScript`
  (locals (Interval :type "Float (double-precision)" :default 0.0))
  (set `local.Interval` (/ (`.MaxTime` (`CurveBase.GetTimeRange` (`self.Curve`))) (`KismetMathLibrary.Conv_IntToDouble` (`self.Count`))))
  (for _index (range (`self.Count`))
    (bind _returnvalue (* _index (`local.Interval`)))
    (bind _returnvalue_2 (`AddComponent|NODE_AddStaticMeshComponent-0` :`RelativeTransform` (`KismetMathLibrary.MakeTransform` (`KismetMathLibrary.MakeVector` _returnvalue 0.0 (`CurveFloat.GetFloatValue` (`self.Curve`) _returnvalue)) (struct) (`KismetMathLibrary.Conv_DoubleToVector` 0.1))))
    (bind _returnvalue_3 (`PrimitiveComponent.CreateDynamicMaterialInstance` _returnvalue_2 0 "/Game/Materials/Mat_Emissive_Sine_Inst.Mat_Emissive_Sine_Inst" "None"))
    (`MaterialInstanceDynamic.SetVectorParameterValue` _returnvalue_3 "Color" (select `int` (mod _index 4) :`0` (struct :`R` 1.0 :`G` 0.010417 :`B` 0.010417 :`A` 1.0) :`1` (struct :`B` 1.0 :`A` 1.0) :`2` (struct :`G` 1.0 :`A` 1.0) :`3` (struct :`R` 1.0 :`G` 1.0 :`A` 1.0) :!type "LinearColor Structure"))))