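; BP_Projectile_Charge is a charged projectile whose strength follows a Scale value, extending a parent projectile Blueprint.
; On BeginPlay it runs the parent logic, then multiplies point light intensity, Damage, Speed and actor size by Scale, keeping Speed above a fixed minimum.
; Overlap and Tick events are disabled, and an unconnected node that would make the box ignore WorldStatic never runs.
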(event `self.ReceiveBeginPlay`
  (`parent.ReceiveBeginPlay`)
  (`LightComponent.SetIntensity` (`self.PointLight`) (* (`self.Intensity`) (`self.Scale`)))
  (set `self.Speed` (`KismetMathLibrary.FMax` (* (`self.Speed`) (`self.Scale`)) 3000.0))
  (set `self.Damage` (* (`self.Damage`) (`self.Scale`)))
  (`self.SetActorScale3D` (* (`self.GetActorScale3D`) (`self.Scale`))))

(fn `UserConstructionScript`
  (`parent.UserConstructionScript`))